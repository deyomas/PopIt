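; Blueprint function library of shared helpers for a dice game.
; It returns the custom game instance, printing a project-settings warning when the cast fails.
; Dice images come from a linear scan of a data table for a row matching value and black flag.
; The score HUD lookup returns the first top-level ScoreBar widget, or nothing when none exists.
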(fn `GetCustomGameInstance`
  (returns (Instance :type "/Game/Blueprints/NewCustomGameInstance Object Reference"))
  (bind _asnew_custom_game_instance (cast `/Game/Blueprints/NewCustomGameInstance` (`GameplayStatics.GetGameInstance` null))
    (:`then`
      (return _asnew_custom_game_instance))
    (:`CastFailed`
      (`KismetSystemLibrary.PrintString` null "You must update the game instance in the project settings")
      (return null))))

(fn `GetDiceImgByNumber`
  (params (Num :type Integer) (Black :type Boolean))
  (returns (Image :type "Texture Object Reference"))
  (locals (DataTable :type "DataTable Object Reference" :default "DataTable'/Game/Blueprints/DiceImages.DiceImages'"))
  (bind _datatable (`local.DataTable`))
  (bind _outrownames (`DataTableFunctionLibrary.GetDataTableRowNames` _datatable))
  (for _array_element _outrownames
    (bind _returnvalue (`|GetDataTableRow` _datatable _array_element)
      (:`then`
        (bind (_image _value _isblack) (break `/Game/Blueprints/Img` _returnvalue))
        (if (and (== Black _isblack) (== Num _value))
          (return _image)))))
  (return null))

(fn `GetScoreHUD`
  (returns (Output :type "/Game/ScoreBar Object Reference"))
  (bind _foundwidgets (`WidgetBlueprintLibrary.GetAllWidgetsOfClass` null "/Game/ScoreBar.ScoreBar_C"))
  (if (> (`KismetArrayLibrary.Array_Length` _foundwidgets) 0)
    (return (`|GetArrayItem` _foundwidgets))
    (else
      (return null))))