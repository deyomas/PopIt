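; NewGameMode is a game mode Blueprint for spawning indexed player characters in what appears to be local multiplayer.
; SpawnPlayer spawns a TopDownCharacter at the given input receiver's transform and has that index's player controller possess it.
; The event graph holds only disconnected logic for tag-matched PlayerStart spawning, local player creation and BP_InputReceiver pawns, so BeginPlay does nothing.
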(event `self.ReceiveBeginPlay`)

(fn `SpawnPlayer`
  (params (IDx :type Integer) (InputRec :type "/Game/BP_InputReceiver Object Reference"))
  (returns (Result :type Boolean))
  (bind _returnvalue (`|SpawnActorFromClass` "/Game/TopDownBP/Blueprints/TopDownCharacter.TopDownCharacter_C" (`self.GetTransform` InputRec) "Undefined" "OverrideRootScale" null IDx null))
  (`Controller.Possess` (`GameplayStatics.GetPlayerController` IDx) _returnvalue))

(fn `UserConstructionScript`)