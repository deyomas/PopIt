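; Custom Game Instance that holds player controller registrations and team data, and puts the score bar on screen.
; RegisterPlayer stores each ID with its gamepad flag and calls Playerregister, while CInit creates the ScoreBar widget once.
; GetTeam searches saved teams by name, otherwise builds a team whose color comes from four defaults, indexed by the name's trailing digit.
; Init and SpawnPlayer are empty, and the CreatePlayer call is disconnected.
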(event `CInit`
  (`/Engine/EditorBlueprintResources/StandardMacros.DoOnce` false
    (:`Completed`
      (bind _returnvalue (`|CreateWidget` "/Game/ScoreBar.ScoreBar_C"))
      (`UserWidget.AddToViewport` _returnvalue 0))))

(event `self.ReceiveInit`)

(event `RegisterPlayer`
  (params (ID :type Integer) (IsGamepad :type Boolean))
  (`BlueprintMapLibrary.Map_Add` (`self.ControllerIDs`) ID IsGamepad)
  (`self.playerregister` ID))

(event `SpawnPlayer`
  (params (PlayerIndex :type Integer) (Pawn :type "Pawn Object Reference")))

(fn `Get Controller IDs`
  (returns (Controllers :type "Array of Integer"))
  (bind _keys (`BlueprintMapLibrary.Map_Keys` (`self.ControllerIDs`)))
  (return _keys))

(fn `GetFirst4DefaultTeamColors`
  (returns (Array :type "Array of SlateColor Structure"))
  (return (`|MakeArray` (make `SlateColor` (struct :`R` 1.0 :`B` 0.061241 :`A` 1.0)) (make `SlateColor` (struct :`R` 0.02247 :`B` 1.0 :`A` 1.0)) (make `SlateColor` (struct :`R` 1.0 :`G` 0.878532 :`A` 1.0)) (make `SlateColor` (struct :`R` 0.062967 :`G` 1.0 :`A` 1.0)))))

(fn `GetTeam`
  (params (TName :type Text))
  (returns (Team :type "/Game/Blueprints/Team Structure") (Found :type Boolean))
  (for _array_element (`self.AllSavedTeams`)
    (if (`KismetTextLibrary.EqualEqual_TextText` (`.TeamName_2_17DDAC7A4A51B84D08CE839568521078` (break `/Game/Blueprints/Team` _array_element)) TName)
      (return _array_element true)))
  (bind _array (`self.GetFirst4DefaultTeamColors`))
  (return (make `/Game/Blueprints/Team` TName (`.SpecifiedColor` (break `SlateColor` (`|GetArrayItem` _array (- (`KismetStringLibrary.Conv_StringToInt` (`KismetStringLibrary.Right` (`KismetTextLibrary.Conv_TextToString` TName) 1)) 1))))) false))