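; GridGenerator is an actor that builds a centred Width by Height grid of PopperSquare actors via its EditorGenerate event.
; EditorGenerate clears the tracked TileList, then spawns, attaches and records each tile relative to the generator's transform.
; GetLocation spaces tiles by side length and gap, and AdjustByCount applies the centring offset.
; X follows the Height index but centres on Width, and vice versa, so only square grids centre correctly.
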(event Custom|EditorGenerate
  (CallFunction|ClearChildren)
  (for _index (range 0 (- (Variables|Default|GetWidth) 1))
    (for _index_2 (range 0 (- (Variables|Default|GetHeight) 1))
      (bind _returnvalue (Game|SpawnActorfromClass "/Game/Blueprints/PopperSquare.PopperSquare_C" (Math|Transform|ComposeTransforms (Math|Transform|MakeTransform (Math|Vector|MakeVector (CallFunction|AdjustbyCount (CallFunction|GetLocation _index_2) (Variables|Default|GetWidth)) (CallFunction|AdjustbyCount (CallFunction|GetLocation _index) (Variables|Default|GetHeight)) 0.0)) (Transformation|GetActorTransform)) "Undefined" 0 0))
      (Transformation|AttachActorToActor _returnvalue self "None" "KeepWorld" "KeepWorld" "KeepWorld" true)
      (Utilities|Array|Add (Variables|Default|GetTileList) _returnvalue))))

(event Custom|ClearChildren
  (bind _tilelist (Variables|Default|GetTileList))
  (for _array_element _tilelist
    (Actor|DestroyActor _array_element))
  (Utilities|Array|Clear _tilelist))

(event EventBeginPlay)

(event Collision|EventActorBeginOverlap
  (params (OtherActor :type Actor%20Object%20Reference)))

(event EventTick
  (params (DeltaSeconds :type Float%20%28single-precision%29)))

(fn ConstructionScript)

(fn GetLocation
  (params (Idx :type Integer))
  (return (|(N*(Len+Space)) (Math|Conversions|ToFloat(Integer) Idx) (Variables|Default|GetTileSideLength) (Variables|Default|GetTileSpacing))))

(fn AdjustbyCount
  (params (Position :type Float%20%28single-precision%29) (Count :type Integer))
  (return (- Position (/ (+ (* (- Count 1) (Variables|Default|GetTileSideLength)) (* (- Count 1) (Variables|Default|GetTileSpacing))) 2.0))))