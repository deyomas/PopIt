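; Board tile that a player ground-pounds to claim for their team and reroll its die value.
; Box overlap checks PlayerInterface for a ground pound and rejects the player's last-claimed tile, then lights the tile.
; Roll tints the dynamic border material and rect light to team color and randomizes the widget's value within the selected die's range.
; It then reports old and new team/value to the score HUD, fires particles and launches the player.
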(event `self.ReceiveBeginPlay`
  (bind _asw_img (`self.GetWImg`))
  (bind _border (`self.Border`))
  (set `self.SidesRange` (select `/Game/Blueprints/DiceSize` (`self.DiceSides`) :`NewEnumerator0` 6 :`NewEnumerator1` 8 :`NewEnumerator2` 12 :`NewEnumerator3` 20))
  (bind _returnvalue (`PrimitiveComponent.CreateDynamicMaterialInstance` _border 1 (`PrimitiveComponent.GetMaterial` _border 1) "None"))
  (set `self.BorderLightMat` _returnvalue)
  (`/Game/W_Img.SetValue` _asw_img (`self.Value`))
  (`/Game/W_Img.SetBlack` _asw_img true)
  (`self.DisableTile`))

(event `self.Box.OnComponentBeginOverlap`
  (params (OverlappedComponent :type "PrimitiveComponent Object Reference") (OtherActor :type "Actor Object Reference") (OtherComp :type "PrimitiveComponent Object Reference") (OtherBodyIndex :type Integer) (bFromSweep :type Boolean) (SweepResult :type "HitResult Structure (by ref)"))
  (if (`KismetSystemLibrary.DoesImplementInterface` OtherActor "/Game/Blueprints/PlayerInterface.PlayerInterface_C")
    (bind _tile (message `/Game/Blueprints/PlayerInterface.GetLastTile` OtherActor))
    (bind _yes (message `/Game/Blueprints/PlayerInterface.IsGroundPounding` OtherActor))
    (if (and _yes (!= _tile self))
      (message `/Game/Blueprints/PlayerInterface.SetLastTile` OtherActor self)
      (`self.EnableTile`)
      (`self.Roll` OtherActor))))

(event `RollDiceAnim`)

(event `ColorTile`
  (params (Value :type "LinearColor Structure"))
  (`MaterialInstanceDynamic.SetVectorParameterValue` (`self.BorderLightMat`) "Color" Value)
  (`LightComponent.SetLightColor` (`self.RectLight1`) Value true)
  (set `self.LastColor` Value))

(event `DisableTile`
  (`self.ColorTile` (struct))
  (`LightComponent.SetIntensity` (`self.RectLight1`) 0.0))

(event `EnableTile`
  (`self.ColorTile` (`self.LastColor`))
  (`LightComponent.SetIntensity` (`self.RectLight1`) 8.0))

(fn `GetWImg`
  (returns (`AsW Img` :type "/Game/W_Img Object Reference"))
  (bind _asw_img (cast `/Game/W_Img` (`WidgetComponent.GetUserWidgetObject` (`self.Widget`))))
  (return _asw_img))

(fn `Roll`
  (params (Player :type "Object Object Reference"))
  (locals (PrevVal :type Integer) (PrevTeam :type Text))
  (bind _instance (`/Game/Blueprints/NewFunctionLibrary.GetCustomGameInstance`))
  (`|ExecutionSequence`
    (:`then_0`
      (set `local.PrevTeam` (`self.CurrentTeam`))
      (bind _teamname (message `/Game/Blueprints/PlayerInterface.GetTeam` Player))
      (set `self.CurrentTeam` _teamname)
      (bind (_team _found) (`/Game/Blueprints/NewCustomGameInstance.GetTeam` _instance _teamname))
      (if _found
        (`self.ColorTile` (`.TeamColor_5_8C87FC9B44BF952F59965BAE5F68DA0F` (break `/Game/Blueprints/Team` _team)))
        (else
          (bind _array (`/Game/Blueprints/NewCustomGameInstance.GetFirst4DefaultTeamColors` _instance))
          (`self.ColorTile` (`.SpecifiedColor` (break `SlateColor` (`|GetArrayItem` _array (`KismetStringLibrary.Conv_StringToInt` (`KismetStringLibrary.Right` (`KismetTextLibrary.Conv_TextToString` _teamname) 1)))))))))
    (:`then_1`
      (set `local.PrevVal` (`self.Value`))
      (set `self.Value` (`KismetMathLibrary.RandomIntegerInRange` 1 (`self.SidesRange`)))
      (`/Game/W_Img.SetValue` (`self.GetWImg`) (`self.Value`)))
    (:`then_2`
      (`/Game/ScoreBar.OnTileChangeValue` (`/Game/Blueprints/NewFunctionLibrary.GetScoreHUD`) (`local.PrevTeam`) (`local.PrevVal`) (`self.CurrentTeam`) (`self.Value`))
      (`ActorComponent.Activate` (`self.ParticleSystem`) true)
      (message `/Game/Blueprints/PlayerInterface.GPLaunch` (`local.Player`)))))

(fn `UserConstructionScript`
  (set `self.Light` (`self.RectLight1`)))